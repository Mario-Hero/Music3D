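; Lyrics display actor that shows a song's LRC lyrics on its LyricUI2 widget, in sync with playback time.
; SetSongPath finds and parses the song's LRC file, tells the Player actor whether lyrics exist, and clears the text when none do.
; UpdateTime passes the current time to UpdateLrc, which looks up the matching line and refreshes the widget only when its index changes or an update is forced.
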(event `self.ReceiveBeginPlay`)

(event `SetSongPath`
  (params (Path :type String))
  (bind _output_get (set `self.SongPath` Path))
  (bind _returnvalue (`LrcReader.FindLrcFile` _output_get))
  (bind _returnvalue_2 (`GameplayStatics.GetActorOfClass` "/Game/Blueprints/Player.Player_C"))
  (`/Engine/EditorBlueprintResources/StandardMacros.IsValid` _returnvalue_2
    (:`Is Valid`
      (bind _returnvalue_3 (`KismetStringLibrary.IsEmpty` _returnvalue))
      (bind _output_get_2 (set `self.HasLrc` (not _returnvalue_3)))
      (`/Game/Blueprints/Player.SetLrcMode` _returnvalue_2 _output_get_2))
    (:`Is Not Valid`
      _))
  (if _returnvalue_3
    (set `self.LrcArray` (`|MakeArray` (struct) :!type "LyricEntry Structure"))
    (bind _aslyric_ui2 (cast `/Game/UI/LyricUI2` (`WidgetComponent.GetWidget` (`self.Widget`))))
    (`/Game/UI/LyricUI2.SetText` _aslyric_ui2 (`|MakeArray` ""))
    (else
      (bind _returnvalue_4 (`LrcReader.ParseLrcFile` _returnvalue))
      (set `self.LrcArray` _returnvalue_4)
      (set `self.Time` 0.0)
      (`self.UpdateLrc` true))))

(event `UpdateTime`
  (params (time :type "Float (double-precision)"))
  (set `self.Time` time)
  (`self.UpdateLrc` false))

(event `UpdateLrc`
  (params (Force :type Boolean))
  (if (`self.HasLrc`)
    (bind _returnvalue (`LrcReader.GetIndexLrc` (`self.LrcArray`) (`self.Time`)))
    (if Force
      (bind _output_get (set `self.index` _returnvalue :!label _label))
      (bind _returnvalue_2 (`LrcReader.GetLrcString` (`self.LrcArray`) _output_get))
      (bind _aslyric_ui2 (cast `/Game/UI/LyricUI2` (`WidgetComponent.GetWidget` (`self.Widget`))))
      (`/Game/UI/LyricUI2.SetText` _aslyric_ui2 _returnvalue_2)
      (elif (not (== _returnvalue (`self.index`)))
        (goto _label)))))

(fn `UserConstructionScript`)