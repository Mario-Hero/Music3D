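; World-space progress bar actor that shows progress through a material parameter and a Bar component moved between Left and Right markers.
; SetProgress eases larger changes with a circular in-out curve on Tick; a looping timer refreshes the bar otherwise.
; Clicking In traces under the mouse, converts hit Y to a fraction and sends it to the Player actor's SetProgress.
; SetColor tints the dynamic material created at construction.
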(event `self.ReceiveBeginPlay`
  (`KismetSystemLibrary.K2_SetTimerDelegate` (delegate `SetProgressOneSecond`) 0.1 true))

(event `SetProgressOneSecond`
  (if (not (`self.Animating`))
    (`self.SetProgressToBar`)))

(event `SetColor`
  (params (Color :type "Color Structure"))
  (`MaterialInstanceDynamic.SetVectorParameterValue` (`self.DynamicMaterial`) "Color" (`KismetMathLibrary.Conv_ColorToLinearColor` Color)))

(event `SetProgress`
  (params (progress :type "Float (double-precision)"))
  (if (not (`self.Animating`))
    (bind _output_get (set `self.ProgressTarget` progress))
    (bind _output_get_2 (set `self.Animating` (> (`KismetMathLibrary.Abs` (- _output_get (`self.Progress`))) 0.1)))
    (if _output_get_2
      (set `self.ProgressStart` (`self.Progress`))
      (set `self.AnimateAlpha` 0.0)
      (else
        (set `self.Progress` (`self.ProgressTarget`))))))

(event `self.ReceiveTick`
  (params (DeltaSeconds :type "Float (single-precision)"))
  (if (`self.Animating`)
    (`self.ProgressLerp` DeltaSeconds)
    (`self.SetProgressToBar`)))

(event `self.in.OnClicked`
  (params (TouchedComponent :type "PrimitiveComponent Object Reference") (ButtonPressed :type "Key Structure"))
  (bind (_worldlocation _worlddirection) (`PlayerController.DeprojectMousePositionToWorld` (`GameplayStatics.GetPlayerController` 0)))
  (bind (_outhit _returnvalue) (`KismetSystemLibrary.LineTraceSingle` :`Start` _worldlocation :`End` (+ _worldlocation (* _worlddirection 1000.0)) :`TraceChannel` "TraceTypeQuery1" :`bIgnoreSelf` false))
  (if _returnvalue
    (bind _progress (`self.Y2Progress` (.y (`.Location` (`GameplayStatics.BreakHitResult` _outhit)))))
    (bind _returnvalue_2 (`GameplayStatics.GetActorOfClass` "/Game/Blueprints/Player.Player_C"))
    (`/Game/Blueprints/Player.SetProgress` _returnvalue_2 _progress)))

(fn `ProgressLerp`
  (params (delta :type "Float (double-precision)"))
  (locals (newProgress :type "Float (double-precision)" :default 0.0))
  (bind _output_get (set `self.AnimateAlpha` (+ (* delta 3.0) (stale _output_get))))
  (set `local.newProgress` (`|EaseFunction` "CircularInOut" _output_get (`self.ProgressStart`) (`self.ProgressTarget`)))
  (if (>= (`self.AnimateAlpha`) 1.0)
    (set `self.Progress` (`self.ProgressTarget`))
    (set `self.Animating` false)
    (set `self.AnimateAlpha` 0.0)
    (else
      (set `self.Progress` (`local.newProgress`)))))

(fn `SetProgressToBar`
  (`MaterialInstanceDynamic.SetScalarParameterValue` (`self.DynamicMaterial`) "progress" (`self.Progress`))
  (`SceneComponent.K2_SetWorldLocation` (`self.Bar`) (`KismetMathLibrary.VLerp` (`SceneComponent.K2_GetComponentLocation` (`self.Left`)) (`SceneComponent.K2_GetComponentLocation` (`self.Right`)) (`self.Progress`)) false true))

(fn `UserConstructionScript`
  (bind (_returnvalue_x _returnvalue_y) (`KismetMathLibrary.BreakVector` (`SceneComponent.K2_GetComponentLocation` (`self.Left`))))
  (bind (_returnvalue_x_2 _returnvalue_y_2) (`KismetMathLibrary.BreakVector` (`SceneComponent.K2_GetComponentLocation` (`self.Right`))))
  (bind _returnvalue (`PrimitiveComponent.CreateDynamicMaterialInstance` (`self.in`) 0 (`self.Material`) "None"))
  (bind _output_get (set `self.DynamicMaterial` _returnvalue))
  (`MaterialInstanceDynamic.SetScalarParameterValue` _output_get "Left" _returnvalue_y)
  (`MaterialInstanceDynamic.SetScalarParameterValue` _output_get "Right" _returnvalue_y_2)
  (`SceneComponent.K2_SetWorldLocation` (`self.Bar`) (`SceneComponent.K2_GetComponentLocation` (`self.Left`)) false true))

(fn `Y2Progress`
  (params (Y :type "Float (double-precision)"))
  (returns (progress :type "Float (double-precision)"))
  (bind (_returnvalue_x _returnvalue_y) (`KismetMathLibrary.BreakVector` (`SceneComponent.K2_GetComponentLocation` (`self.Right`))))
  (bind (_returnvalue_x_2 _returnvalue_y_2) (`KismetMathLibrary.BreakVector` (`SceneComponent.K2_GetComponentLocation` (`self.Left`))))
  (return (/ (- Y _returnvalue_y_2) (- _returnvalue_y _returnvalue_y_2))))