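; Music player actor that plays a shuffled folder playlist, importing each file at runtime through RuntimeAudioImporter as a 2D sound.
; Finished tracks advance the playlist, and pause, seek, stop and insertion are supported.
; Playback drives scene actors for progress, times, lyrics, volume and title, while cached MP3 tags or cover files supply artwork whose main color tints controls.
; Tick eases cover and title between lyric and no-lyric layouts.
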(event `self.ReceiveBeginPlay`
  (bind _returnvalue (`RuntimeAudioImporterLibrary.CreateRuntimeAudioImporter`))
  (set `self.Importer` _returnvalue))

(event `AddDir`
  (params (Dir :type String))
  (set `self.MusicFolder` Dir)
  (bind _returnvalue (`FunctionLibrary.GetAllMusicInFolder` (`self.MusicFolder`)))
  (bind _output_get (set `self.MusicList` _returnvalue))
  (`KismetArrayLibrary.Array_Shuffle` _output_get)
  (`self.ChangeSong` 0))

(event `ChangeSong`
  (params (IndexChange :type Integer))
  (bind _track (`self.track`))
  (bind _importer (`self.Importer`))
  (if (> (`KismetArrayLibrary.Array_Length` (`self.MusicList`)) 0)
    (if (not (`self.ChangingSong`))
      (set `self.ChangingSong` true)
      (`VolumeControl.UpdateSoundWave` (`self.VolumeControl`) null)
      (`/Engine/EditorBlueprintResources/StandardMacros.IsValid` _track
        (:`Is Valid`
          (clear `AudioComponent.OnAudioPlaybackPercent` _track)
          (clear `AudioComponent.OnAudioFinished` _track)
          (`AudioComponent.Stop` _track))
        (:`Is Not Valid`
          _))
      (set `self.PlayIndex` (mod (+ IndexChange (`self.PlayIndex`)) (`KismetArrayLibrary.Array_Length` (`self.MusicList`))))
      (bind _output_get (set `self.MusicPath` (`|GetArrayItem` (`self.MusicList`) (`self.PlayIndex`))))
      (`KismetSystemLibrary.PrintString` _output_get)
      (if (`BlueprintPathsLibrary.FileExists` _output_get)
        (`/Engine/EditorBlueprintResources/StandardMacros.IsValid` _importer
          (:`Is Valid`
            _)
          (:`Is Not Valid`
            (bind _returnvalue (`RuntimeAudioImporterLibrary.CreateRuntimeAudioImporter`))
            (set `self.Importer` _returnvalue)))
        (add `RuntimeAudioImporterLibrary.OnResult` _importer (delegate `OnResult`))
        (`RuntimeAudioImporterLibrary.ImportAudioFromFile` _importer _output_get "Auto")
        (else
          (`KismetSystemLibrary.PrintString` "file not exist"))))))

(event `PlayFinish`
  (`self.ChangeSong` 1))

(event `OnResult`
  (params (Importer :type "RuntimeAudioImporterLibrary Object Reference") (ImportedSoundWave :type "ImportedSoundWave Object Reference") (Status :type "ERuntimeImportStatus Enum" :default "SuccessfulImport"))
  (set `self.ChangingSong` false)
  (if (`|EnumEquality` Status "SuccessfulImport")
    (bind _output_get (set `self.Sound` ImportedSoundWave))
    (`/Game/Blueprints/lyrics.SetSongPath` (`self.Lyrics`) (`self.MusicPath`))
    (bind _returnvalue (`GameplayStatics.CreateSound2D` _output_get 1.0 1.0 0.0 null false false))
    (bind _output_get_2 (set `self.track` _returnvalue))
    (`VolumeControl.UpdateSoundWave` (`self.VolumeControl`) _output_get_2)
    (set `self.ProgressStart` 0.0)
    (add `AudioComponent.OnAudioPlaybackPercent` _output_get_2 (delegate `ProgressBarChange`))
    (add `AudioComponent.OnAudioFinished` _output_get_2 (delegate `PlayFinish`))
    (`/Game/Blueprints/AllTime2D.SetTime` (`self.AllTime`) (`KismetMathLibrary.FTrunc` (`SoundBase.Duration` (`self.Sound`))))
    (`AudioComponent.Play` _output_get_2 0.0)
    (bind _returnvalue_2 (`self.InfoGetter`))
    (`self.CoverOperation` (`.cover` (break `MusicTag` _returnvalue_2)))
    (`/Game/Blueprints/TitleArtist.SetInfo` (`self.TitleInfo`) _returnvalue_2)
    (else
      (`KismetSystemLibrary.PrintString` (`KismetStringLibrary.Conv_ByteToString` Status)))))

(event `ProgressBarChange`
  (params (PlayingSoundWave :type "SoundWave Object Reference") (PlaybackPercent :type "Float (double-precision)"))
  (bind _returnvalue (+ (`self.ProgressStart`) PlaybackPercent))
  (bind _returnvalue_2 (`GameplayStatics.GetActorOfClass` "/Game/Blueprints/ProgressBar.ProgressBar_C"))
  (bind _output_get (set `self.realTime` (* _returnvalue (`SoundBase.Duration` PlayingSoundWave))))
  (`/Game/Blueprints/ProgressBar.SetProgress` _returnvalue_2 _returnvalue)
  (`/Game/Blueprints/PlayTime2D.SetTime` (`self.PlayTime`) (`KismetMathLibrary.FTrunc` _output_get))
  (`/Game/Blueprints/lyrics.UpdateTime` (`self.Lyrics`) _output_get))

(event `Pause`
  (params (bPause :type Boolean))
  (bind _track (`self.track`))
  (`/Engine/EditorBlueprintResources/StandardMacros.IsValid` _track
    (:`Is Valid`
      (`AudioComponent.SetPaused` _track bPause))))

(event `SetProgress`
  (params (NewProgress :type "Float (double-precision)"))
  (bind _track (`self.track`))
  (`/Engine/EditorBlueprintResources/StandardMacros.IsValid` _track
    (:`Is Valid`
      (set `self.ChangingSong` true)
      (clear `AudioComponent.OnAudioFinished` _track)
      (`AudioComponent.Stop` _track)
      (`KismetSystemLibrary.Delay` 0.1)
      (set `self.ProgressStart` NewProgress)
      (`AudioComponent.Play` _track (* NewProgress (`SoundBase.Duration` (`self.Sound`))))
      (set `self.ChangingSong` false)
      (add `AudioComponent.OnAudioFinished` _track (delegate `PlayFinish`)))))

(event `SetLrcMode`
  (params (HasLrc :type Boolean))
  (if (not (== HasLrc (`self.HasLrc`)))
    (set `self.LrcAnimating` true)
    (set `self.HasLrc` HasLrc)))

(event `self.ReceiveTick`
  (params (DeltaSeconds :type "Float (single-precision)"))
  (bind (_loca _locb _rota _rotb _scalea _scaleb) (`self.LrcAnimatingCoverLocRot`))
  (bind (_loca_2 _locb_2 _rota_2 _rotb_2 _scalea_2 _scaleb_2) (`self.LrcAnimatingTitleLocRot`))
  (bind _cover (`self.Cover`))
  (bind _titleinfo (`self.TitleInfo`))
  (bind _lrcanimateprogress (`self.LrcAnimateProgress`))
  (if (`self.LrcAnimating`)
    (bind _output_get (set `self.LrcAnimateProgress` (+ (stale _output_get) (* DeltaSeconds 4.0))))
    (`self.K2_SetActorLocationAndRotation` _cover (`|EaseFunction` "EaseInOut" _output_get _loca _locb) (`|EaseFunction` "EaseInOut" _output_get _rota _rotb) false false)
    (`self.SetActorScale3D` _cover (`|EaseFunction` "EaseInOut" _output_get _scalea _scaleb))
    (`self.K2_SetActorLocationAndRotation` _titleinfo (`|EaseFunction` "EaseInOut" _lrcanimateprogress _loca_2 _locb_2) (`|EaseFunction` "EaseInOut" _lrcanimateprogress _rota_2 _rotb_2) false true)
    (`self.SetActorScale3D` _titleinfo (`|EaseFunction` "EaseInOut" _lrcanimateprogress _scalea_2 _scaleb_2))
    (if (> (`self.LrcAnimateProgress`) 1.0)
      (set `self.LrcAnimating` false)
      (set `self.LrcAnimateProgress` 0.0)
      (`self.SetCoverTitleLocRot`))))

(event `Stop`
  (bind _track (`self.track`))
  (`/Engine/EditorBlueprintResources/StandardMacros.IsValid` _track
    (:`Is Valid`
      (clear `AudioComponent.OnAudioFinished` _track)
      (`AudioComponent.Stop` _track))))

(event `AddMusic`
  (params (path :type String))
  (`KismetArrayLibrary.Array_Insert` (`self.MusicList`) path (+ (`self.PlayIndex`) 1)))

(fn `CacheInfo`
  (params (path :type String) (tag :type "MusicTag Structure"))
  (bind _cacheinfomap (`self.CacheInfoMap`))
  (`BlueprintMapLibrary.Map_Add` _cacheinfomap path tag)
  (if (> (`BlueprintMapLibrary.Map_Length` _cacheinfomap) 50)
    (bind _keys (`BlueprintMapLibrary.Map_Keys` _cacheinfomap))
    (`BlueprintMapLibrary.Map_Remove` _cacheinfomap (`KismetArrayLibrary.Array_Random` _keys))))

(fn `CoverOperation`
  (params (cover :type "Texture2D Object Reference"))
  (`/Game/Blueprints/Cover.SetCover` (`self.Cover`) cover)
  (`/Engine/EditorBlueprintResources/StandardMacros.IsValid` cover
    (:`Is Valid`
      (bind _returnvalue (`FunctionLibrary.GetMainColor` cover))
      (bind _output_get (set `self.CoverMainColor` _returnvalue))
      (`/Game/Blueprints/ProgressBar.SetColor` (`self.ProgressBar`) _output_get)
      (`/Game/Blueprints/PausePlay.SetColor` (`self.PausePlay`) (`KismetMathLibrary.Conv_ColorToLinearColor` _output_get)))))

(fn `GetVariables`
  (bind _returnvalue (`GameplayStatics.GetActorOfClass` "/Game/Blueprints/Cover.Cover_C"))
  (set `self.Cover` _returnvalue)
  (bind _returnvalue_2 (`GameplayStatics.GetActorOfClass` "/Game/Blueprints/ProgressBar.ProgressBar_C"))
  (set `self.ProgressBar` _returnvalue_2)
  (bind _returnvalue_3 (`GameplayStatics.GetActorOfClass` "/Game/Blueprints/PlayTime2D.PlayTime2D_C"))
  (set `self.PlayTime` _returnvalue_3)
  (bind _returnvalue_4 (`GameplayStatics.GetActorOfClass` "/Game/Blueprints/PausePlay.PausePlay_C"))
  (set `self.PausePlay` _returnvalue_4)
  (bind _returnvalue_5 (`GameplayStatics.GetActorOfClass` "/Game/Blueprints/TitleArtist.TitleArtist_C"))
  (set `self.TitleInfo` _returnvalue_5)
  (bind _returnvalue_6 (`GameplayStatics.GetActorOfClass` "/Game/Blueprints/lyrics.lyrics_C"))
  (set `self.Lyrics` _returnvalue_6)
  (bind _returnvalue_7 (`GameplayStatics.GetActorOfClass` "/Game/Blueprints/AllTime2D.AllTime2D_C"))
  (set `self.AllTime` _returnvalue_7)
  (bind _returnvalue_8 (`GameplayStatics.GetActorOfClass` "/Script/Music3D.VolumeControl"))
  (set `self.VolumeControl` _returnvalue_8))

(fn `InfoGetter`
  (returns (ReturnValue :type "MusicTag Structure"))
  (locals (info :type "MusicTag Structure"))
  (bind _musicpath (`self.MusicPath`))
  (bind (_title _artist _album _comment _genre _year _track _cover) (break `MusicTag` (`local.info`)))
  (bind (_value _returnvalue) (`BlueprintMapLibrary.Map_Find` (`self.CacheInfoMap`) _musicpath))
  (if _returnvalue
    (return _value)
    (else
      (bind _returnvalue_2 (`TagLib.GetMP3Tag` _musicpath))
      (bind _output_get (set `local.info` _returnvalue_2))
      (if (`KismetStringLibrary.IsEmpty` _title)
        (setmembers `MusicTag` :`StructRef` _output_get :`title` (`BlueprintPathsLibrary.GetBaseFilename` _musicpath)))
      (`/Engine/EditorBlueprintResources/StandardMacros.IsValid` _cover
        (:`Is Valid`
          _)
        (:`Is Not Valid`
          (bind _returnvalue_3 (`FunctionLibrary.FindCoverFile` (`self.MusicPath`)))
          (if (`KismetStringLibrary.IsEmpty` _returnvalue_3)
            (`KismetSystemLibrary.PrintString` "Cannot find cover")
            (else
              (bind _returnvalue_4 (`FunctionLibrary.LoadTexture2D` _returnvalue_3))
              (setmembers `MusicTag` :`StructRef` (`local.info`) :`cover` _returnvalue_4)))))
      (`self.CacheInfo` (`self.MusicPath`) (`local.info`))
      (return (`local.info`)))))

(fn `LrcAnimatingCoverLocRot`
  (returns (LocA :type "Vector Structure") (LocB :type "Vector Structure") (RotA :type "Rotator Structure") (RotB :type "Rotator Structure") (ScaleA :type "Vector Structure") (ScaleB :type "Vector Structure"))
  (bind _nolrccoverloc (`self.NoLrcCoverLoc`))
  (bind _lrccoverloc (`self.LrcCoverLoc`))
  (bind _lrccoverrot (`self.LrcCoverRot`))
  (bind _nolrccoverrot (`self.NoLrcCoverRot`))
  (bind _nolrccoverscale (`self.NoLrcCoverScale`))
  (bind _lrccoverscale (`self.LrcCoverScale`))
  (if (`self.HasLrc`)
    (return _nolrccoverloc _lrccoverloc _nolrccoverrot _lrccoverrot _nolrccoverscale _lrccoverscale)
    (else
      (return _lrccoverloc _nolrccoverloc _lrccoverrot _nolrccoverrot _lrccoverscale _nolrccoverscale))))

(fn `LrcAnimatingTitleLocRot`
  (returns (LocA :type "Vector Structure") (LocB :type "Vector Structure") (RotA :type "Rotator Structure") (RotB :type "Rotator Structure") (ScaleA :type "Vector Structure") (ScaleB :type "Vector Structure"))
  (bind _lrctitlerot (`self.LrcTitleRot`))
  (bind _nolrctitlescale (`self.NoLrcTitleScale`))
  (bind _lrctitlescale (`self.LrcTitleScale`))
  (bind _nolrctitleloc (`self.NoLrcTitleLoc`))
  (bind _lrctitleloc (`self.LrcTitleLoc`))
  (bind _nolrctitlerot (`self.NoLrcTitleRot`))
  (if (`self.HasLrc`)
    (return _nolrctitleloc _lrctitleloc _nolrctitlerot _lrctitlerot _nolrctitlescale _lrctitlescale)
    (else
      (return _lrctitleloc _nolrctitleloc _lrctitlerot _nolrctitlerot _lrctitlescale _nolrctitlescale))))

(fn `SetCoverTitleLocRot`
  (bind (_loca _locb _rota _rotb _scalea _scaleb) (`self.LrcAnimatingCoverLocRot`))
  (bind (_loca_2 _locb_2 _rota_2 _rotb_2 _scalea_2 _scaleb_2) (`self.LrcAnimatingTitleLocRot`))
  (bind _cover (`self.Cover`))
  (bind _titleinfo (`self.TitleInfo`))
  (`self.K2_SetActorLocationAndRotation` _cover _locb _rotb false false)
  (`self.SetActorScale3D` _cover _scaleb)
  (`self.K2_SetActorLocationAndRotation` _titleinfo _locb_2 _rotb_2 false false)
  (`self.SetActorScale3D` _titleinfo _scaleb_2))

(fn `UserConstructionScript`
  (`self.GetVariables`)
  (`self.SetCoverTitleLocRot`))