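; Cover actor that displays a picture from a supplied texture, or a Music placeholder when none is given, with an animated swap between covers.
; SetCover flips a Switch between two component sets, updating the incoming set's dynamic material and visibility.
; Tick slides the old cover out and the new one in with circular easing.
; Otherwise, the active cover tilts toward the viewport mouse position while hovered and eases back afterward.
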(event `SetCover`
  (params (texture :type "Texture2D Object Reference"))
  (bind _returnvalue (`KismetSystemLibrary.IsValid` texture))
  (bind _output_get (set `self.Switch` (not (stale _output_get))))
  (if _returnvalue
    (`MaterialInstanceDynamic.SetTextureParameterValue` (`self.GetDynmaterial`) "Texture" texture))
  (`SceneComponent.SetVisibility` (`self.GetPicture`) _returnvalue false)
  (`SceneComponent.SetVisibility` (`self.GetMusic`) (not _returnvalue) false)
  (set `self.Animating` true)
  (`SceneComponent.SetVisibility` (`.CoverIn` (`self.GetCoverBoth`)) true false))

(event `self.ReceiveTick`
  (params (DeltaSeconds :type "Float (single-precision)"))
  (bind (_coverout _coverin) (`self.GetCoverBoth`))
  (bind _relativelocation (`SceneComponent.RelativeLocation` (`self.LocNormal`)))
  (if (`self.Animating`)
    (bind _output_get (set `self.AnimateProgress` (+ (stale _output_get) (* DeltaSeconds 2.0))))
    (`SceneComponent.K2_SetRelativeLocation` _coverout (`|EaseFunction` "CircularInOut" _output_get _relativelocation (`SceneComponent.RelativeLocation` (`self.LocOut`))) false true)
    (`SceneComponent.K2_SetRelativeLocation` _coverin (`|EaseFunction` "CircularInOut" _output_get (`SceneComponent.RelativeLocation` (`self.LocIn`)) _relativelocation) false true)
    (if (> _output_get 1.0)
      (set `self.Animating` false)
      (set `self.AnimateProgress` 0.0)
      (`SceneComponent.SetVisibility` (`self.GetCoverBoth`) false false))
    (else
      (`self.FollowMouseFun`))))

(event `self.Box.OnBeginCursorOver`
  (params (TouchedComponent :type "PrimitiveComponent Object Reference"))
  (set `self.FollowMouse` true :!label _label))

(event `self.Box.OnEndCursorOver`
  (params (TouchedComponent :type "PrimitiveComponent Object Reference"))
  (set `self.FollowMouse` false :!label _label_2))

(event `self.Box1.OnBeginCursorOver`
  (params (TouchedComponent :type "PrimitiveComponent Object Reference"))
  (goto _label))

(event `self.Box1.OnEndCursorOver`
  (params (TouchedComponent :type "PrimitiveComponent Object Reference"))
  (goto _label_2))

(fn `FollowMouseFun`
  (bind _picture (`self.GetPicture`))
  (bind _music (`self.GetMusic`))
  (bind _relativerotation (`SceneComponent.RelativeRotation` _picture))
  (bind _relativerotation_2 (`SceneComponent.RelativeRotation` _music))
  (if (`self.FollowMouse`)
    (bind _target (`self.MouseOnCover`))
    (`SceneComponent.K2_SetRelativeRotation` _picture (`KismetMathLibrary.RLerp` _relativerotation (`FunctionLibrary.AddRotatorDirect` _target (`self.PictureRotationOri`)) 0.4 true) false false)
    (`SceneComponent.K2_SetRelativeRotation` _music (`KismetMathLibrary.RLerp` _relativerotation_2 (`FunctionLibrary.AddRotatorDirect` _target (`self.MusicRotationOri`)) 0.4 true) false false)
    (else
      (`SceneComponent.K2_SetRelativeRotation` _picture (`KismetMathLibrary.RLerp` _relativerotation (`self.PictureRotationOri`) 0.1 true) false false)
      (`SceneComponent.K2_SetRelativeRotation` _music (`KismetMathLibrary.RLerp` _relativerotation_2 (`self.MusicRotationOri`) 0.1 true) false false))))

(fn `GetCoverBoth`
  (returns (CoverOut :type "SceneComponent Object Reference") (CoverIn :type "SceneComponent Object Reference"))
  (bind _cover (`self.Cover`))
  (bind _cover1 (`self.Cover1`))
  (if (`self.Switch`)
    (return _cover _cover1)
    (else
      (return _cover1 _cover))))

(fn `GetDynmaterial`
  (returns (DynMaterial :type "MaterialInstanceDynamic Object Reference"))
  (if (`self.Switch`)
    (return (`self.DynMaterial1`))
    (else
      (return (`self.DynMaterial`)))))

(fn `GetMusic`
  (returns (music :type "StaticMeshComponent Object Reference"))
  (if (`self.Switch`)
    (return (`self.Music1`))
    (else
      (return (`self.Music`)))))

(fn `GetPicture`
  (returns (picture :type "StaticMeshComponent Object Reference"))
  (if (`self.Switch`)
    (return (`self.picture1`))
    (else
      (return (`self.picture`)))))

(fn `MouseOnCover`
  (returns (Target :type "Rotator Structure"))
  (bind (_returnvalue_x _returnvalue_y) (`KismetMathLibrary.BreakVector2D` (`WidgetLayoutLibrary.GetViewportSize`)))
  (bind _returnvalue (`WidgetLayoutLibrary.GetMousePositionOnViewport`))
  (return (`KismetMathLibrary.MakeRotator` (* 1 (/ (- (`.Y` (`KismetMathLibrary.BreakVector2D` _returnvalue)) (/ _returnvalue_y 3.0)) 150.0)) 0.0 (* -1 (/ (- (`KismetMathLibrary.BreakVector2D` _returnvalue) (/ _returnvalue_x 4.0)) 150.0)))))

(fn `UserConstructionScript`
  (bind _returnvalue (`PrimitiveComponent.CreateDynamicMaterialInstance` (`self.picture`) 0 (`self.Material`) "None"))
  (set `self.DynMaterial` _returnvalue)
  (bind _returnvalue_2 (`PrimitiveComponent.CreateDynamicMaterialInstance` (`self.picture1`) 0 (`self.Material`) "None"))
  (set `self.DynMaterial1` _returnvalue_2)
  (set `self.PictureRotationOri` (`SceneComponent.RelativeRotation` (`self.picture`)))
  (set `self.MusicRotationOri` (`SceneComponent.RelativeRotation` (`self.Music`)))
  (`SceneComponent.SetVisibility` (`self.GetPicture`) false false)
  (`SceneComponent.SetVisibility` (`self.GetMusic`) true false))