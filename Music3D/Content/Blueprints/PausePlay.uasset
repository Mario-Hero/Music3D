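; PausePlay is the 3D transport control for the music player, with play/pause, next and previous buttons.
; Collider clicks or Space and arrow keys call Pause or ChangeSong on the Player actor found by class.
; Tick drives eased animations: a "Play" morph target for the play/pause icon and a scale pulse on the pressed skip button.
; SetColor tints the Play mesh through a dynamic material created in the construction script.
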(event `self.ReceiveTick`
  (params (DeltaSeconds :type "Float (single-precision)"))
  (`self.PlayPauseSwitchFun` DeltaSeconds)
  (`self.PlayButtonAnimate` DeltaSeconds))

(event `InputAction|Space`
  (params (Key :type "Key Structure"))
  (:`Pressed`
    (`self.SwitchTo` (not (`self.nowPlaying`)) :!label _label)))

(event `self.PlayColl.OnClicked`
  (params (TouchedComponent :type "PrimitiveComponent Object Reference") (ButtonPressed :type "Key Structure"))
  (goto _label))

(event `SwitchTo`
  (params (`play?` :type Boolean))
  (bind _output_get (set `self.nowPlaying` `play?`))
  (set `self.progress` 0.0)
  (set `self.playpauseswitching` true)
  (bind _returnvalue (`GameplayStatics.GetActorOfClass` "/Game/Blueprints/Player.Player_C"))
  (`/Game/Blueprints/Player.Pause` _returnvalue (not _output_get)))

(event `SetColor`
  (params (Color :type "LinearColor Structure"))
  (set `self.Color` Color)
  (`MaterialInstanceDynamic.SetVectorParameterValue` (`self.Dynmaterial`) "Color" Color))

(event `InputAction|KeyRight`
  (params (Key :type "Key Structure"))
  (:`Pressed`
    (bind _returnvalue (`GameplayStatics.GetActorOfClass` "/Game/Blueprints/Player.Player_C" :!label _label_2))
    (`/Game/Blueprints/Player.ChangeSong` _returnvalue 1)
    (set `self.PlayButtonAnimating` (make `/Game/Blueprints/AnimateStruct` true true 0.0 (`self.Next`)))))

(event `self.NextColl.OnClicked`
  (params (TouchedComponent :type "PrimitiveComponent Object Reference") (ButtonPressed :type "Key Structure"))
  (goto _label_2))

(event `self.PreviousColl.OnClicked`
  (params (TouchedComponent :type "PrimitiveComponent Object Reference") (ButtonPressed :type "Key Structure"))
  (bind _returnvalue (`GameplayStatics.GetActorOfClass` "/Game/Blueprints/Player.Player_C" :!label _label_3))
  (`/Game/Blueprints/Player.ChangeSong` _returnvalue -1)
  (set `self.PlayButtonAnimating` (make `/Game/Blueprints/AnimateStruct` true true 0.0 (`self.Previous`))))

(event `InputAction|KeyLeft`
  (params (Key :type "Key Structure"))
  (:`Pressed`
    (goto _label_3)))

(fn `PlayButtonAnimate`
  (params (delta :type "Float (double-precision)"))
  (bind _playbuttonanimating (`self.PlayButtonAnimating`))
  (bind (_animating _goup _progress) (break `/Game/Blueprints/AnimateStruct` _playbuttonanimating))
  (bind (_animating_2 _goup_2 _progress_2 _mesh) (break `/Game/Blueprints/AnimateStruct` (`self.PlayButtonAnimating`)))
  (bind (_animating_3 _goup_3 _progress_3 _mesh_2) (break `/Game/Blueprints/AnimateStruct` (`self.PlayButtonAnimating`)))
  (if _animating
    (setmembers `/Game/Blueprints/AnimateStruct` :`StructRef` _playbuttonanimating :`Progress` (+ _progress (* delta 5.0)))
    (if (> _progress_3 1.0)
      (if _goup_2
        (set `self.PlayButtonAnimating` (make `/Game/Blueprints/AnimateStruct` true false 0.0 _mesh))
        (else
          (`SceneComponent.SetRelativeScale3D` _mesh (0.3 0.3 0.3))
          (set `self.PlayButtonAnimating` (make `/Game/Blueprints/AnimateStruct` false))))
      (else
        (`SceneComponent.SetRelativeScale3D` _mesh_2 (* (0.3 0.3 0.3) (`FunctionLibrary.LerpLimit` 1.0 2.0 (`|EaseFunction` "CircularInOut" _progress 0.0 1.0) _goup)))))))

(fn `PlayPauseSwitchFun`
  (params (A :type "Float (double-precision)"))
  (if (`self.playpauseswitching`)
    (bind _returnvalue (+ (* A 3.0) (stale _output_get)))
    (bind _output_get (set `self.progress` _returnvalue))
    (if (> (`self.progress`) 1.0)
      (set `self.playpauseswitching` false)
      (else
        (`SkeletalMeshComponent.SetMorphTarget` (`self.Play`) "Play" (`FunctionLibrary.LerpLimit` 0.0 1.0 (`|EaseFunction` "CircularInOut" _returnvalue 0.0 1.0) (not (`self.nowPlaying`))) true)))))

(fn `UserConstructionScript`
  (bind _returnvalue (`PrimitiveComponent.CreateDynamicMaterialInstance` (`self.Play`) 0 null "None"))
  (set `self.Dynmaterial` _returnvalue))