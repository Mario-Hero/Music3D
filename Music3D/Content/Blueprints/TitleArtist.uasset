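; TitleArtist is an actor Blueprint that displays a title and artist name through two widget components.
; Its SetInfo event takes an Info struct, casts the Title component's widget to TitleInfoUI and the Artist component's to ArtistInfoUI, then sets each text from the matching field.
; A failed Title cast also skips the artist update, and no other event contains logic.
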(event `SetInfo`
  (params (Info :type "MusicTag Structure"))
  (bind (_title _artist) (break `MusicTag` Info))
  (bind _astitle_info_ui (cast `/Game/UI/TitleInfoUI` (`WidgetComponent.GetUserWidgetObject` (`self.Title`))))
  (`/Game/UI/TitleInfoUI.SetText` _astitle_info_ui (`KismetTextLibrary.Conv_StringToText` _title))
  (bind _asartist_info_ui (cast `/Game/UI/ArtistInfoUI` (`WidgetComponent.GetUserWidgetObject` (`self.Artist`))))
  (`/Game/UI/ArtistInfoUI.SetText` _asartist_info_ui (`KismetTextLibrary.Conv_StringToText` _artist)))

(fn `UserConstructionScript`)