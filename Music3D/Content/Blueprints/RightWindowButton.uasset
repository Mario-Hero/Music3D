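; Actor that provides clickable quit, maximize and minimize window buttons through QuitBox, MaxBox and MinBox components.
; Quit calls Stop on the Player actor before exiting, and minimize calls SetWindowMinimize.
; PressMaxBox toggles between windowed and windowed fullscreen via GameUserSettings, saving the windowed resolution to restore later.
; It also swaps visibility of the Window and Max components to reflect the mode.
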(event `self.QuitBox.OnClicked`
  (params (TouchedComponent :type "PrimitiveComponent Object Reference") (ButtonPressed :type "Key Structure"))
  (bind _returnvalue (`GameplayStatics.GetActorOfClass` "/Game/Blueprints/Player.Player_C"))
  (`/Game/Blueprints/Player.Stop` _returnvalue)
  (`KismetSystemLibrary.QuitGame` null "Quit"))

(event `self.MaxBox.OnClicked`
  (params (TouchedComponent :type "PrimitiveComponent Object Reference") (ButtonPressed :type "Key Structure"))
  (`self.PressMaxBox`))

(event `self.MinBox.OnClicked`
  (params (TouchedComponent :type "PrimitiveComponent Object Reference") (ButtonPressed :type "Key Structure"))
  (`WindowLibrary.SetWindowMinimize`))

(fn `PressMaxBox`
  (locals (`Windowed?` :type Boolean))
  (bind _returnvalue (`GameUserSettings.GetGameUserSettings`))
  (bind _output_get (set `local.Windowed?` (`|EnumEquality` (`GameUserSettings.GetFullscreenMode` _returnvalue) "Windowed")))
  (if _output_get
    (bind _output_get_2 (set `self.WindowRes` (`GameUserSettings.GetScreenResolution` _returnvalue)))
    (`GameUserSettings.SetFullscreenMode` _returnvalue "WindowedFullscreen")
    (`GameUserSettings.ApplySettings` _returnvalue false)
    (else
      (`GameUserSettings.SetFullscreenMode` _returnvalue "Windowed")
      (`GameUserSettings.SetScreenResolution` _returnvalue _output_get_2)
      (`GameUserSettings.ApplySettings` _returnvalue false)))
  (`SceneComponent.SetVisibility` (`self.Window`) _output_get false)
  (`SceneComponent.SetVisibility` (`self.Max`) (not _output_get) false))

(fn `UserConstructionScript`)